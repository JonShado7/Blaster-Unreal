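; BP_Creature_AI is the AI controller for BP_Creature.
; On possess it caches the creature and runs the BT_Creature behavior tree.
; AI perception updates for Character_Blueprint write whether it was successfully sensed to the "Can See Player?" blackboard key.
; Walk and Run events forward to the creature's functions of the same name and print debug strings.
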(event `self.AIPerception.OnTargetPerceptionUpdated`
  (params (Actor :type "Actor Object Reference") (Stimulus :type "AIStimulus Structure"))
  (cast `/Game/Blueprints/Character_Blueprint` Actor)
  (`BlackboardComponent.SetValueAsBool` (`AIBlueprintHelperLibrary.GetBlackboard` null) "Can See Player?" (`.bSuccessfullySensed` (break `AIStimulus` Stimulus))))

(event `Walk`
  (`/Game/Blueprints/AI/FirstAI/BP_Creature.Walk` (`self.Creature`))
  (`KismetSystemLibrary.PrintString` "Being Fucking Called"))

(event `Run`
  (`/Game/Blueprints/AI/FirstAI/BP_Creature.Run` (`self.Creature`))
  (`KismetSystemLibrary.PrintString` "Fuck Yess"))

(event `self.OnPossess`
  (params (PossessedPawn :type "Pawn Object Reference"))
  (bind _asbp_creature (cast `/Game/Blueprints/AI/FirstAI/BP_Creature` PossessedPawn))
  (set `self.Creature` _asbp_creature)
  (`self.RunBehaviorTree` "/Game/Blueprints/AI/FirstAI/BT_Creature.BT_Creature"))

(fn `UserConstructionScript`)