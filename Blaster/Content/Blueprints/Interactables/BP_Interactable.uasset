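; BP_Interactable is an interactable actor that makes itself known to the player character when it comes within range.
; Overlaps on InteractableArea register the actor with Character_Blueprint on begin, along with a debug print, and unregister it on end.
; SetHighlight toggles custom depth rendering on InteractableMesh to switch its highlight on or off; nothing in this Blueprint calls it.
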(event `self.Interactable Area.OnComponentBeginOverlap`
  (params (OverlappedComponent :type "PrimitiveComponent Object Reference") (OtherActor :type "Actor Object Reference") (OtherComp :type "PrimitiveComponent Object Reference") (OtherBodyIndex :type Integer) (bFromSweep :type Boolean) (SweepResult :type "HitResult Structure (by ref)"))
  (bind _ascharacter_blueprint (cast `/Game/Blueprints/Character_Blueprint` OtherActor))
  (message `/Game/Blueprints/Interactables/BPI_Interact.Register Interactable` _ascharacter_blueprint self)
  (`KismetSystemLibrary.PrintString` "Hello"))

(event `self.Interactable Area.OnComponentEndOverlap`
  (params (OverlappedComponent :type "PrimitiveComponent Object Reference") (OtherActor :type "Actor Object Reference") (OtherComp :type "PrimitiveComponent Object Reference") (OtherBodyIndex :type Integer))
  (bind _ascharacter_blueprint (cast `/Game/Blueprints/Character_Blueprint` OtherActor))
  (message `/Game/Blueprints/Interactables/BPI_Interact.UnRegister Interactable` _ascharacter_blueprint self))

(fn `Set Highlight`
  (params (Highlight :type Boolean))
  (`PrimitiveComponent.SetRenderCustomDepth` (`self.Interactable Mesh`) Highlight))

(fn `UserConstructionScript`)