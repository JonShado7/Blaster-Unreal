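; BP_GameMode is a game mode Blueprint that copies player state from the player's Character_Blueprint into its own variables.
; On BeginPlay it calls GetPlayerHealth, which casts player character 0 and stores its CurrentHealth as a one-time snapshot.
; A similar GetInventory function copies the character's Inventory and InventorySize, but nothing in this file calls it.
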(event `self.ReceiveBeginPlay`
  (`self.Get Player Health`))

(fn `Get Inventory`
  (bind _ascharacter_blueprint (cast `/Game/Blueprints/Character_Blueprint` (`GameplayStatics.GetPlayerCharacter` 0)))
  (set `self.Inventory` (`/Game/Blueprints/Character_Blueprint.Inventory` _ascharacter_blueprint))
  (set `self.Inventory Size` (`/Game/Blueprints/Character_Blueprint.InventorySize` _ascharacter_blueprint)))

(fn `Get Player Health`
  (bind _ascharacter_blueprint (cast `/Game/Blueprints/Character_Blueprint` (`GameplayStatics.GetPlayerCharacter` 0)))
  (set `self.Player Health` (`/Game/Blueprints/Character_Blueprint.Current Health` _ascharacter_blueprint)))

(fn `UserConstructionScript`)